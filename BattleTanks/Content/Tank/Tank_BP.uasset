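; Player tank Blueprint that drives on two tracks, aims and fires, and shows a health bar.
; BeginPlay hands barrel, turret and tracks to TankAiming and TankMovement, then gives the health bar widget a tank reference.
; Input rotates the spring arm and gimbal for frame-rate-scaled aiming, and fires through TankAiming.
; Movement sets track throttles directly, opposed for turning, bypassing unused TankMovement calls; MoveBack drives only the right track.
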(event EventBeginPlay
  (bind _tankaiming (Variables|Default|GetTankAiming))
  (Class|TankAimingComponent|SetBarrel _tankaiming (Variables|Default|GetBarrel))
  (Class|TankAimingComponent|SetTurrent _tankaiming (Variables|Default|GetTurrent))
  (Class|TankMovementComponent|SetTracks (Variables|Default|GetTankMovement) (Variables|Default|GetL%20Track) (Variables|Default|GetR%20Track))
  (CallFunction|InitializeHealthBar))

(event Input|ActionEvents|InputActionFire
  (params (Key :type Key%20Structure :default "AnyKey"))
  ;[1 1 1] Input Binding
  ;;[1 1 1] Fire!
  (:Pressed
    (Class|TankAimingComponent|Fire (Variables|Default|GetTankAiming))))

(event Input|AxisEvents|InputAxisAimAzimuth
  (params (AxisValue :type Float%20%28single-precision%29))
  ;[1 1 1] Input Binding
  ;;[1 1 1] Aiming
  (Transformation|AddLocalRotation (Variables|Default|GetSpringArm) (Math|Rotator|MakeRotator 0.0 0.0 (* (Utilities|Time|GetWorldDeltaSeconds) AxisValue 1e+02)) false false))

(event Input|AxisEvents|InputAxisMoveBack
  (params (AxisValue :type Float%20%28single-precision%29))
  ;[1 1 1] Input Binding
  ;;[1 1 1] Move Back
  (Class|Tank|MoveTrack (Variables|Default|GetR%20Track) AxisValue))

(event Input|AxisEvents|InputAxisMoveForward
  (params (AxisValue :type Float%20%28single-precision%29))
  ;[1 1 1] Input Binding
  ;;[1 1 1] Move Forward
  (Class|Tank|MoveTrack (Variables|Default|GetL%20Track) AxisValue)
  (Class|Tank|MoveTrack (Variables|Default|GetR%20Track) AxisValue))

(event Input|AxisEvents|InputAxisMoveLeft
  (params (AxisValue :type Float%20%28single-precision%29))
  ;[1 1 1] Input Binding
  ;;[1 1 1] Move Left (Right Track)
  (Class|Tank|MoveTrack (Variables|Default|GetR%20Track) AxisValue)
  (Class|Tank|MoveTrack (Variables|Default|GetL%20Track) (* AxisValue -1.0)))

(event Input|AxisEvents|InputAxisMoveRight
  (params (AxisValue :type Float%20%28single-precision%29))
  ;[1 1 1] Input Binding
  ;;[1 1 1] Move Right (Left Track)
  (Class|Tank|MoveTrack (Variables|Default|GetL%20Track) AxisValue)
  (Class|Tank|MoveTrack (Variables|Default|GetR%20Track) (* AxisValue -1.0)))

(event Input|AxisEvents|InputAxisAimElevation
  (params (AxisValue :type Float%20%28single-precision%29))
  ;[1 1 1] Input Binding
  ;;[1 1 1] Aiming
  (Transformation|AddLocalRotation (Variables|Default|GetAzimuth%20Gimbal) (Math|Rotator|MakeRotator 0.0 (* AxisValue (Utilities|Time|GetWorldDeltaSeconds) 1e+02) 0.0) false false))

(fn ConstructionScript)

(fn InitializeHealthBar
  (bind _ashealth_bar_bp (Utilities|Casting|CastToHealthBar_BP (UserInterface|GetUserWidgetObject (Variables|Default|GetWidget))))
  (Variables|/Game/UI/HealthBar_BP.HealthBar_BP_C|SetTankReference _ashealth_bar_bp self)
  (return))